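; Paintable canvas actor that lets callers stamp brush textures onto its surface and wipe it back to white.
; On BeginPlay it creates a white render target, feeds it into a dynamic M_PaintCanvas material on the Canvas component, and creates a dynamic brush material.
; DrawOntoCanvas sets the brush texture and draws that material into the render target, centered on a normalized location at a pixel size.
; ClearPaintCanvas refills the target with white.
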(event `self.ReceiveBeginPlay`
  (`|ExecutionSequence`
    (:`then_0`
      (bind _returnvalue (`KismetRenderingLibrary.CreateRenderTarget2D` 1024 1024))
      (bind _output_get (set `self.RenderTarget` _returnvalue))
      (`KismetRenderingLibrary.ClearRenderTarget2D` _output_get (struct :`R` 1.0 :`G` 1.0 :`B` 1.0 :`A` 1.0)))
    (:`then_1`
      (bind _returnvalue_2 (`KismetMaterialLibrary.CreateDynamicMaterialInstance` "/Game/Nixon/Canvas/PaintCanvasMaterial/M_PaintCanvas.M_PaintCanvas"))
      (`MaterialInstanceDynamic.SetTextureParameterValue` _returnvalue_2 "RenderTarget" (`self.RenderTarget`))
      (`PrimitiveComponent.SetMaterial` (`self.Canvas`) 0 _returnvalue_2))
    (:`then_2`
      (bind _returnvalue_3 (`KismetMaterialLibrary.CreateDynamicMaterialInstance` "/Game/Nixon/Canvas/PaintCanvasMaterial/M_BrushMat.M_BrushMat"))
      (set `self.Brushmaterial` _returnvalue_3))))

(event `self.DrawOntoCanvas`
  (params (tex2d :type "Texture2D Object Reference") (brush_size :type "Float (single-precision)") (draw_location :type "Vector2D Structure"))
  (`self.DrawBrush` tex2d brush_size draw_location))

(event `self.ClearPaintCanvas`
  (`self.ClearCanvas`))

(fn `ClearCanvas`
  (`KismetRenderingLibrary.ClearRenderTarget2D` (`self.RenderTarget`) (struct :`R` 1.0 :`G` 1.0 :`B` 1.0 :`A` 1.0)))

(fn `DrawBrush`
  (params (BrushTexture :type "Texture2D Object Reference") (brushSize :type "Float (double-precision)") (DrawLocation :type "Vector2D Structure"))
  (locals (DrawLoc :type "Vector2D Structure") (BrushSizeLocal :type "Float (double-precision)"))
  (bind _brushsize (`local.brushSize`))
  (set `local.BrushSizeLocal` brushSize)
  (set `local.DrawLoc` DrawLocation)
  (`|ExecutionSequence`
    (:`then_0`
      (`MaterialInstanceDynamic.SetTextureParameterValue` (`self.Brushmaterial`) "BrushTexture" BrushTexture))
    (:`then_1`
      (bind (_canvas _size _context) (`KismetRenderingLibrary.BeginDrawCanvasToRenderTarget` (`self.RenderTarget`)))
      (`Canvas.K2_DrawMaterial` _canvas (`self.Brushmaterial`) (- (* _size (`local.DrawLoc`)) (/ _brushsize 2.0)) (`KismetMathLibrary.MakeVector2D` _brushsize _brushsize) (0.0 0.0) (1.0 1.0) 0.0 (0.5 0.5))
      (`KismetRenderingLibrary.EndDrawCanvasToRenderTarget` _context))))

(fn `UserConstructionScript`)